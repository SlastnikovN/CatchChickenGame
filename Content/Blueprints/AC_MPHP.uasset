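; AC_MPHP is an actor component that stores current and maximum HP and MP values for its owner.
; Setter functions write the max values together and each current value separately, with no clamping.
; GetStatsForHUD returns all four values as truncated integer text, plus HP and MP progress-bar fractions normalized against their maximums.
; It has no active event logic, so other code drives every change.
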(event EventBeginPlay)

(event EventTick
  (params (DeltaSeconds :type Float%20%28single-precision%29)))

(fn GetStatsforHUD
  (return (Utilities|Text|ToText(Integer) (Math|Float|Truncate (Variables|Default|GetMaxHP))) (Utilities|Text|ToText(Integer) (Math|Float|Truncate (Variables|Default|GetCurrentHP))) (Math|Float|NormalizetoRange (Variables|Default|GetCurrentHP) 0.0 (Variables|Default|GetMaxHP)) (Utilities|Text|ToText(Integer) (Math|Float|Truncate (Variables|Default|GetMaxMP))) (Utilities|Text|ToText(Integer) (Math|Float|Truncate (Variables|Default|GetCurrentMP))) (Math|Float|NormalizetoRange (Variables|Default|GetCurrentMP) 0.0 (Variables|Default|GetMaxMP))))

(fn SetMAXHPMaxMP
  (params (MaxHP :type Float%20%28double-precision%29) (MaxMP :type Float%20%28double-precision%29))
  (Variables|Default|SetMaxHP MaxHP)
  (Variables|Default|SetMaxMP MaxMP))

(fn SetCurrentHP
  (params (CurrentHP :type Float%20%28double-precision%29))
  (Variables|Default|SetCurrentHP CurrentHP))

(fn SetCurrentMP
  (params (CurrentMP :type Float%20%28double-precision%29))
  (Variables|Default|SetCurrentMP CurrentMP))