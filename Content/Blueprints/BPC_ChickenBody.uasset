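; Chicken character that the player catches by touching its capsule, which awards points through the player's AddChickenMessage and destroys the chicken.
; The player entering its detection sphere plays a timeline that drives MaxWalkSpeed, with a delay on the update that later zeroes the speed.
; The end-overlap check compares the overlapped component, not the other actor, with the player, so anything leaving the sphere reverses the timeline.
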(event OnComponentHit(CapsuleComponent)
  (params (HitComponent :type Primitive%20Component%20Object%20Reference) (OtherActor :type Actor%20Object%20Reference) (OtherComp :type Primitive%20Component%20Object%20Reference) (NormalImpulse :type Vector :default "0, 0, 0") (Hit :type Hit%20Result%20Structure%20%28by%20ref%29))
  ;[1 1 1] Удаление курицы со сцены и назначение очков игроку
  (if (== OtherActor (Game|GetPlayerCharacter 0))
    (Class|BPICharacter|AddChicken(Message) (Game|GetPlayerCharacter 0) 5)
    (Actor|DestroyActor)))

(event OnComponentBeginOverlap(Sphere)
  (params (OverlappedComponent :type Primitive%20Component%20Object%20Reference) (OtherActor :type Actor%20Object%20Reference) (OtherComp :type Primitive%20Component%20Object%20Reference) (OtherBodyIndex :type Integer) (bFromSweep :type Boolean) (SweepResult :type Hit%20Result%20Structure%20%28by%20ref%29))
  (bind _charactermovement (Variables|Character|GetCharacterMovement))
  (if (== OtherActor (Game|GetPlayerCharacter 0))
    (bind _newtrack_0 (Timeline|TimelineWalkAndRun Play)
      (:Update
        (Variables|/Script/Engine.CharacterMovementComponent|SetMaxWalkSpeed _charactermovement _newtrack_0)
        (Utilities|FlowControl|Delay 7.0)
        (Variables|/Script/Engine.CharacterMovementComponent|SetMaxWalkSpeed _charactermovement 0.0)))))

(event OnComponentEndOverlap(Sphere)
  (params (OverlappedComponent :type Primitive%20Component%20Object%20Reference) (OtherActor :type Actor%20Object%20Reference) (OtherComp :type Primitive%20Component%20Object%20Reference) (OtherBodyIndex :type Integer))
  (bind _charactermovement (Variables|Character|GetCharacterMovement))
  (if (not (== OverlappedComponent (Game|GetPlayerCharacter 0)))
    (bind _newtrack_0 (Timeline|TimelineWalkAndRun Reverse)
      (:Update
        (Variables|/Script/Engine.CharacterMovementComponent|SetMaxWalkSpeed _charactermovement _newtrack_0)
        (Utilities|FlowControl|Delay 7.0)
        (Variables|/Script/Engine.CharacterMovementComponent|SetMaxWalkSpeed _charactermovement 0.0)))))

(fn ConstructionScript)